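; MamaFireFly_BP is a firefly boss enemy that tracks its health and shows it on the player's boss health bar.
; It sets current health to total at construction and fetches the player's health bar widget a second after BeginPlay.
; LoseHealthTick subtracts damage per tick, updates the bar percentage, and calls Death at zero, though that event is empty here.
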(event `self.ReceiveBeginPlay`
  ;[1 0.01026 0] BEGINPLAY
  (`KismetSystemLibrary.Delay` 1.0)
  (set `self.HealthWidget` (`/Game/FirstPersonBP/Blueprints/FirstPersonCharacter.HealthBarsWidget` (`self.Player`))))

(event `LoseHealthTick`
  (params (DamagePerTick :type "Float (double-precision)"))
  ;[0.3139 1 0] LOSE HEALTH TICK
  (bind _output_get (set `self.CurrentHP` (- (`self.CurrentHP`) DamagePerTick)))
  (`ProgressBar.SetPercent` (`/Game/HUD/HealthBars_Widget.BossHealthBar` (`self.HealthWidget`)) (/ _output_get (`self.TotalHP`)))
  (if (<= _output_get 0.0)
    (`self.Death`)))

(event `Death`)

(fn `UserConstructionScript`
  (set `self.CurrentHP` (`self.TotalHP`)))