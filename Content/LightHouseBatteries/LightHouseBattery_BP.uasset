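; Lighthouse battery Blueprint that accumulates charge and shows its progress with six internal particle systems.
; Each GetCharge call adds the given per-second rate scaled by world delta time to the current charge.
; When the charge ratio exceeds the next threshold, it activates that stage's particle system, advances the stage and raises the threshold by about a sixth, clamped at full.
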(event Custom|GetCharge
  (params (BatteryCargePSec :type Float%20%28single-precision%29))
  (Variables|Default|SetCurrentBatteryCharge (+ (* BatteryCargePSec (Utilities|Time|GetWorldDeltaSeconds)) (Variables|Default|GetCurrentBatteryCharge)))
  (Utilities|FlowControl|Sequence
    (:then_0
      ;[1 1 1] PARTICLE SYSTEMS INSIDE LIGHT UP
      (if (|((A/B)>X) (Variables|Default|GetPercentageForNext) (Variables|Default|GetCurrentBatteryCharge) (Variables|Default|GetBatteryChargeNeeded))
        (Utilities|FlowControl|Sequence
          (:then_0
            (switch int (Variables|Default|GetbatteryStage)
              (:0
                (Components|Activation|SetActive (Variables|Default|GetBatterParticleSystem) true false))
              (:1
                (Components|Activation|SetActive (Variables|Default|GetBatterParticleSystem2) true false))
              (:2
                (Components|Activation|SetActive (Variables|Default|GetBatterParticleSystem3) true false))
              (:3
                (Components|Activation|SetActive (Variables|Default|GetBatterParticleSystem4) true false))
              (:4
                (Components|Activation|SetActive (Variables|Default|GetBatterParticleSystem5) true false))
              (:5
                (Components|Activation|SetActive (Variables|Default|GetBatterParticleSystem6) true false))))
          (:then_1
            (Math|Integer|IncrementInt (Variables|Default|GetbatteryStage)))
          (:then_2
            (Variables|Default|SetPercentageForNext (Math|Float|Clamp(Float) (+ (Variables|Default|GetPercentageForNext) (Math|Float|MakeLiteralFloat 0.166667))))))))))

(fn ConstructionScript)