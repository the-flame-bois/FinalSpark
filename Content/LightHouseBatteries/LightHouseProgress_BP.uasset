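; Lighthouse progress manager that counts charged batteries to unlock the fight entrance and trigger the game's ending.
; BeginPlay creates the progress widget, and each BatteryCharged event plays audio, increments the count and updates the widget's jars.
; At six charges it removes the barriers and opens the fight entrance; at twelve it disables input and plays the ending sequence at triple speed.
; Tick polls for the sequence to finish, then loads the main menu.
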(event `self.ReceiveBeginPlay`
  (bind _returnvalue (`|CreateWidget` "/Game/HUD/LighthouseProgress_Widget.LighthouseProgress_Widget_C" (`GameplayStatics.GetPlayerController` 0)))
  (`UserWidget.AddToViewport` _returnvalue 0)
  (set `self.widget` _returnvalue))

(event `BatteryCharged`
  (bind _returnvalue (`GameplayStatics.GetPlayerController` 0))
  (bind _sequenceplayer (`LevelSequenceActor.SequencePlayer` (`self.endingScene`)))
  (`AudioComponent.Play` (`self.Audio`) 0.0)
  (bind _result (`/Engine/EditorBlueprintResources/StandardMacros.IncrementInt` (`self.NumOfCompleted`))
    (:`  `
      (`/Game/HUD/LighthouseProgress_Widget.JarFilled` (`self.widget`))
      (if (== _result 6)
        (for _array_element (`self.barriers`)
          (`self.SetActorHiddenInGame` _array_element true)
          (`self.SetActorEnableCollision` _array_element false)
          (set `/Game/EnemyBoss/EntranceToFightTrigger.canPLayerEnter` true (`self.entranceToFight`)))
        (elif (== _result 12)
          (`self.DisableInput` _returnvalue _returnvalue)
          (`MovieSceneSequencePlayer.SetPlayRate` _sequenceplayer 3.0)
          (`MovieSceneSequencePlayer.Play` _sequenceplayer)
          (set `self.hasEnded` true))))))

(event `self.ReceiveTick`
  (params (DeltaSeconds :type "Float (single-precision)"))
  (if (`self.hasEnded`)
    (if (not (`MovieSceneSequencePlayer.IsPlaying` (`LevelSequenceActor.SequencePlayer` (`self.endingScene`))))
      (`GameplayStatics.OpenLevel` "MainMenu"))))

(fn `UserConstructionScript`)