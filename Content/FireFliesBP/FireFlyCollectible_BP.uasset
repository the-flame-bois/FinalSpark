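; Firefly collectible that wanders around its start point and can be sucked toward the player.
; A looping or one-shot MovementTimeline offsets and yaws the mesh, scaled by MoveRange and MoveSpeed.
; StartSuck halts wandering and runs SuckTimeline, scaling the actor and pulling the mesh toward the player's FireFlyStream.
; StopSuck reverses that timeline and resumes wandering, while completing it hides the firefly and disables collision.
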(event `self.ReceiveBeginPlay`
  ;[1 0 0.07823] BEGINPLAY
  (set `self.InitialLoc` (`SceneComponent.RelativeLocation` (`self.Mesh`)))
  (`TimelineComponent.SetPlayRate` (`self.MovementTimeline`) (`self.MoveSpeed`))
  (bind (_direction _x _y _z _rotz) (`Timeline|MovementTimeline` :!label _label)
    (:`Update`
      (`SceneComponent.K2_SetRelativeLocation` (`self.Mesh`) (+ (* (`KismetMathLibrary.MakeVector` _x _y _z) (`self.MoveRange`)) (`self.InitialLoc`)) false false)
      (`SceneComponent.K2_SetRelativeRotation` (`self.Mesh`) (`KismetMathLibrary.MakeRotator` 0.0 0.0 (* _rotz 90.0)) false false))))

(event `StartSuck`
  (params (Player :type "/Game/FirstPersonBP/Blueprints/FirstPersonCharacter Object Reference"))
  ;[1 0.9447 0] SUCC
  (`|ExecutionSequence`
    (:`then_0`
      (set `self.Player` Player)
      (if (not (`self.isBeingSucked`))
        (set `self.PreSuckLoc` (`SceneComponent.K2_GetComponentLocation` (`self.Mesh`)))))
    (:`then_1`
      (goto _label :!via `Stop`))
    (:`then_2`
      (set `self.isBeingSucked` true))
    (:`then_3`
      (bind (_direction _sizealpha _distance_alpha) (`Timeline|SuckTimeline` :!label _label_2)
        (:`Update`
          (`SceneComponent.SetWorldScale3D` (`self.DefaultSceneRoot`) (`KismetMathLibrary.MakeVector` _sizealpha _sizealpha _sizealpha))
          (`SceneComponent.K2_SetWorldLocation` (`self.Mesh`) (`KismetMathLibrary.VLerp` (`SceneComponent.K2_GetComponentLocation` (`/Game/FirstPersonBP/Blueprints/FirstPersonCharacter.FireFlyStream` (`self.Player`))) (`self.PreSuckLoc`) _distance_alpha) false false))
        (:`Finished`
          (switch `ETimelineDirection` _direction
            (:`Forward`
              (`self.FinishSuck`))
            (:`Backward`
              (`|ExecutionSequence`
                (:`then_0`
                  (set `self.isBeingSucked` false))
                (:`then_1`
                  (goto _label))))))))))

(event `StopSuck`
  ;[1 1 1] stop suc
  (if (`self.isBeingSucked`)
    (goto _label_2 :!via `Reverse`)))

(event `FinishSuck`
  ;[0 1 0.02964] SUCCED
  (`self.SetActorEnableCollision` false)
  (`self.SetActorHiddenInGame` true))

(fn `UserConstructionScript`)